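; TestCityBP is a blocking prop that procedurally fills a square grid with placeholder skyscrapers.
; The construction script loops from -HalfSize to HalfSize on X and Y, placing one instance every Spacing units.
; A RandomStream picks one of three skyscraper instanced mesh components and a uniform scale variation for each cell, so layouts are repeatable per seed.
; The event graph is unused.
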(fn `UserConstructionScript`
  (locals (WorkingTransform :type "Transform Structure"))
  (bind _spacing (`self.Spacing`))
  (bind _halfsize (`self.HalfSize`))
  (bind _returnvalue (* -1 _halfsize))
  (for _index (range _returnvalue (+ _halfsize 1))
    (for _index_2 (range _returnvalue (+ _halfsize 1))
      (set `local.WorkingTransform` (`KismetMathLibrary.MakeTransform` (`KismetMathLibrary.MakeVector` (* _index _spacing) (* _index_2 _spacing)) (struct) (* (1.0 1.0 1.0) (`KismetMathLibrary.RandomFloatInRangeFromStream` 0.8 1.2 (`self.RandomStream`)))))
      (`InstancedStaticMeshComponent.AddInstance` (select `int` (`KismetMathLibrary.RandomIntegerInRangeFromStream` 0 2 (`self.RandomStream`)) :`0` (`self.SkyscraperA`) :`1` (`self.SkyscraperB`) :`2` (`self.SkyscraperC`) :!type "InstancedStaticMeshComponent Object Reference") (`local.WorkingTransform`)))))